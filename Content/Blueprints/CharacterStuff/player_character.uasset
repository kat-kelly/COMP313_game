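; Player character Blueprint handling keyboard movement, mouse look and a double jump.
; Axis inputs feed MovementFB and MovementLR, which move the character relative to control yaw; mouse X turns the controller while mouse Y pitches CameraArm directly.
; A DoN counter on Space triggers Jump, then an additive upward LaunchCharacter, and resets on landing.
; Disconnected climbing nodes (hang montage, capsule move to a ledge) remain in the graph but never run.
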(event `Key|SpaceBar`
  (params (Key :type "Key Structure"))
  ;[1 1 1] character movement: keyboard
  (:`Pressed`
    (bind _counter (`/Engine/EditorBlueprintResources/StandardMacros.Do N` 2 :!label _label)
      (:`Exit`
        (switch `int` _counter
          (:`1`
            (`self.Jump`))
          (:`2`
            (`self.LaunchCharacter` (0.0 0.0 300.0))))))))

(event `self.OnLanded`
  (params (Hit :type "HitResult Structure (by ref)"))
  ;[1 1 1] character movement: keyboard
  (goto _label :!via `Reset`))

(event `InputAxis|Forward`
  (params (AxisValue :type "Float (single-precision)"))
  ;[1 1 1] character movement: keyboard
  (`self.MovementFB` AxisValue))

(event `InputAxis|Back`
  (params (AxisValue :type "Float (single-precision)"))
  ;[1 1 1] character movement: keyboard
  (`self.MovementFB` AxisValue))

(event `InputAxis|Left`
  (params (AxisValue :type "Float (single-precision)"))
  ;[1 1 1] character movement: keyboard
  (`self.MovementLR` AxisValue))

(event `InputAxis|Right`
  (params (AxisValue :type "Float (single-precision)"))
  ;[1 1 1] character movement: keyboard
  (`self.MovementLR` AxisValue))

(event `InputAxisKey|MouseX`
  (params (AxisValue :type "Float (single-precision)"))
  ;[1 1 1] character movement: mouse
  (`self.AddControllerYawInput` AxisValue))

(event `InputAxisKey|MouseY`
  (params (AxisValue :type "Float (single-precision)"))
  ;[1 1 1] character movement: mouse
  (`SceneComponent.K2_AddRelativeRotation` (`self.camera arm`) (`KismetMathLibrary.MakeRotator` 0.0 AxisValue) false false))

(event `self.ReceiveTick`
  (params (DeltaSeconds :type "Float (single-precision)")))

(fn `MovementFB`
  (params (ScaleValue :type "Float (double-precision)"))
  (`self.AddMovementInput` self (`KismetMathLibrary.GetForwardVector` (`KismetMathLibrary.MakeRotator` 0.0 0.0 (.yaw (`self.GetControlRotation`)))) ScaleValue true))

(fn `MovementLR`
  (params (ScaleValue :type "Float (double-precision)"))
  (`self.AddMovementInput` self (`KismetMathLibrary.GetRightVector` (`KismetMathLibrary.MakeRotator` 0.0 0.0 (.yaw (`self.GetControlRotation`)))) ScaleValue true))

(fn `UserConstructionScript`)